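; Procedurally spawned room that registers with the game mode, populates itself with enemies and unlocks its exit door once they are dead.
; Tagged mesh components mark enemy and chest spawn points and are hidden on construction; chests are not spawned here.
; A DoN loop spawns a random, minimum-bounded number of fixed or random-class enemies at non-repeating points.
; RegisterEnemyDeath empties the tracked list, then RoomCleared unlocks the door spawned at ExitPoint.
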(event `StartRoomConstruction`
  (`/Game/Core/BP_CustomGameMode.AddSpawnedRoomToArray` (`/Game/Core/BPFL_MainLibrary.Get Main Game Mode`) self)
  (bind _possibleenemyspawns (`self.Get All Possible Enemy Spawns`))
  (`self.MakeEveryActorOfArrayInvisible` _possibleenemyspawns)
  (bind _possiblechestspawns (`self.Get All Possible Chest Spawns`))
  (`self.MakeEveryActorOfArrayInvisible` _possiblechestspawns)
  (`self.Spawn Enemies At Possible Spawn Locations`))

(event `SpawnDoorAtExitPoint`
  (bind (_returnvalue_location _returnvalue_rotation) (`KismetMathLibrary.BreakTransform` (`SceneComponent.K2_GetComponentToWorld` (`self.ExitPoint`))))
  (bind _returnvalue (`|SpawnActorFromClass` "/Game/Procedural/BP_Door.BP_Door_C" (`KismetMathLibrary.MakeTransform` _returnvalue_location _returnvalue_rotation) "Undefined" "OverrideRootScale" null null))
  (set `self.AssociatedDoor` _returnvalue))

(event `RoomCleared`
  (`KismetSystemLibrary.PrintString` "Room Cleared" true true (struct :`R` 1.0 :`B` 0.017152 :`A` 1.0))
  (`/Game/Procedural/BP_Door.UnlockDoor` (`self.AssociatedDoor`)))

(fn `AllEnemiesEliminated`
  (returns (ReturnValue :type Boolean))
  (return (== (`KismetArrayLibrary.Array_Length` (`self.SpawnedEnemies`)) 0)))

(fn `Get All Possible Chest Spawns`
  (returns (PossibleChestSpawns :type "Array of StaticMeshComponent Object Reference"))
  (bind _output_get (set `self.PossibleChestSpawns` (`self.GetComponentsByTag` "/Script/Engine.StaticMeshComponent" "ChestSpawn")))
  (return _output_get))

(fn `Get All Possible Enemy Spawns`
  (returns (PossibleEnemySpawns :type "Array of StaticMeshComponent Object Reference"))
  (bind _output_get (set `self.PossibleEnemySpawns` (`self.GetComponentsByTag` "/Script/Engine.StaticMeshComponent" "EnemySpawn")))
  (return _output_get))

(fn `GetRandomArrayObject`
  (params (Array :type "Array of StaticMeshComponent Object Reference"))
  (returns (RandomArrayObject :type "StaticMeshComponent Object Reference") (RandomArrayObjectTransform :type "Transform Structure"))
  (bind _outitem (`KismetArrayLibrary.Array_Random` Array))
  (return _outitem (`SceneComponent.K2_GetComponentToWorld` _outitem)))

(fn `GetRandomEnemyAmount`
  (returns (RandomEnemyAmount :type Integer))
  (bind _returnvalue (`KismetArrayLibrary.Array_Length` (`self.PossibleEnemySpawns`)))
  (return (`KismetMathLibrary.RandomIntegerInRange` (`KismetMathLibrary.Clamp` (`self.MinimumEnemiesAmount`) 0 _returnvalue) _returnvalue)))

(fn `GetRandomEnemyClass`
  (returns (RandomEnemyClass :type "Actor Class Reference"))
  (return (`KismetArrayLibrary.Array_Random` (`self.PossibleEnnemyClasses`))))

(fn `MakeEveryActorOfArrayInvisible`
  (params (Array :type "Array of StaticMeshComponent Object Reference"))
  (for _array_element Array
    (`SceneComponent.SetHiddenInGame` _array_element true true)
    (`PrimitiveComponent.SetCollisionResponseToAllChannels` _array_element "ECR_Ignore")))

(fn `RegisterEnemyDeath`
  (params (EnemyThatDied :type "/Game/Enemies/BP_Enemy Object Reference (by ref)"))
  (`KismetArrayLibrary.Array_RemoveItem` (`self.SpawnedEnemies`) EnemyThatDied)
  (if (`self.AllEnemiesEliminated`)
    (`self.RoomCleared`)))

(fn `Spawn Enemies At Possible Spawn Locations`
  (locals (SelectedRandomSpawnPoint :type "StaticMeshComponent Object Reference") (EnnemiesToSpawnLOCAL :type Integer :default 0))
  (bind _output_get (set `local.EnnemiesToSpawnLOCAL` (`self.GetRandomEnemyAmount`)))
  (`/Engine/EditorBlueprintResources/StandardMacros.Do N` _output_get :!label _label
    (:`Exit`
      (bind _output_get_2 (set `local.SelectedRandomSpawnPoint` (`self.GetRandomArrayObject` (`self.PossibleEnemySpawns`))))
      (bind (_returnvalue_location _returnvalue_rotation) (`KismetMathLibrary.BreakTransform` (`SceneComponent.K2_GetComponentToWorld` _output_get_2)))
      (`|SpawnActorFromClass` (select `bool` (`self.SingleEnemyType`) :`false` (`self.GetRandomEnemyClass`) :`true` (`self.SingleEnemyTypeClass`) :!type "Actor Class Reference") (`KismetMathLibrary.MakeTransform` _returnvalue_location _returnvalue_rotation) "Undefined" "OverrideRootScale" null null)
      (`KismetArrayLibrary.Array_Add` (`self.SpawnedEnemies`) null)
      (`KismetArrayLibrary.Array_RemoveItem` (`self.PossibleEnemySpawns`) (`local.SelectedRandomSpawnPoint`))
      (goto _label))))

(fn `SpawnActorsAtLocation`
  (params (ActorToSpawn :type "Actor Class Reference") (SpawnTransform :type "Transform Structure")))

(fn `UserConstructionScript`)