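; Loot chest that, the first time it is interacted with, ejects one to three random items, the count rolled at BeginPlay.
; A DoN loop with half-second delays spawns a BP_ItemSpawner per item at ItemSpawnPoint, using a random class from PossibleItemsInChest.
; LaunchItemSpawner tosses each upward and outward with a velocity impulse, fanned by count and index.
; The debug print re-rolls the random pick, so it can differ from the spawned item.
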(event `self.ReceiveBeginPlay`
  (set `self.ItemsToSpawnAmount` (`KismetMathLibrary.RandomIntegerInRange` 1 3)))

(event `/Game/Core/BPI_Interact.OnInteracted`
  (params (Player :type "/Game/Core/BP_FirstPersonCharacter Object Reference"))
  (`/Engine/EditorBlueprintResources/StandardMacros.DoOnce` false
    (:`Completed`
      (`self.SpawnSequence`))))

(event `SpawnSequence`
  (bind _outitem (`KismetArrayLibrary.Array_Random` (`self.PossibleItemsInChest`)))
  (bind _counter (`/Engine/EditorBlueprintResources/StandardMacros.Do N` (`self.ItemsToSpawnAmount`) :!label _label)
    (:`Exit`
      (bind _returnvalue (`|SpawnActorFromClass` "/Game/Gameplay/BP_ItemSpawner.BP_ItemSpawner_C" (`KismetMathLibrary.MakeTransform` (`SceneComponent.K2_GetComponentLocation` (`self.ItemSpawnPoint`))) "Undefined" "OverrideRootScale" null _outitem null))
      (`KismetSystemLibrary.PrintString` (`KismetSystemLibrary.GetClassDisplayName` _outitem))
      (`self.LaunchItemSpawner` _returnvalue (`self.ItemsToSpawnAmount`) _counter)
      (`KismetSystemLibrary.Delay` 0.5)
      (goto _label))))

(fn `GetLaunchForwardVector`
  (returns (ReturnValue :type "Vector Structure"))
  (return (`KismetMathLibrary.MakeVector` (.x (* (`self.GetActorForwardVector`) 150.0)) (.y (* (`self.GetActorForwardVector`) 150.0)) (+ (.z (* (`self.GetActorForwardVector`) 150.0)) 375.0))))

(fn `GetLaunchLeftVector`
  (returns (ReturnValue :type "Vector Structure"))
  (return (`KismetMathLibrary.MakeVector` (.x (* (+ (`self.GetActorForwardVector`) (`self.GetActorRightVector`)) 150.0)) (.y (* (+ (`self.GetActorForwardVector`) (`self.GetActorRightVector`)) 150.0)) (+ (.z (* (+ (`self.GetActorForwardVector`) (`self.GetActorRightVector`)) 150.0)) 375.0))))

(fn `GetLaunchRightVector`
  (returns (ReturnValue :type "Vector Structure"))
  (return (`KismetMathLibrary.MakeVector` (.x (* (+ (`self.GetActorForwardVector`) (* (`self.GetActorRightVector`) -1.0)) 150.0)) (.y (* (+ (`self.GetActorForwardVector`) (* (`self.GetActorRightVector`) -1.0)) 150.0)) (+ (.z (* (+ (`self.GetActorForwardVector`) (* (`self.GetActorRightVector`) -1.0)) 150.0)) 375.0))))

(fn `LaunchItemSpawner`
  (params (ItemSpawner :type "/Game/Gameplay/BP_ItemSpawner Object Reference") (TotalItemsAmount :type Integer) (CurrentItemIndex :type Integer))
  (switch `int` TotalItemsAmount
    (:`1`
      (`PrimitiveComponent.AddImpulse` (`/Game/Gameplay/BP_ItemSpawner.Sphere` (`local.ItemSpawner`)) (`self.GetLaunchForwardVector`) "None" true))
    (:`2`
      (`PrimitiveComponent.AddImpulse` (`/Game/Gameplay/BP_ItemSpawner.Sphere` (`local.ItemSpawner`)) (select `int` CurrentItemIndex :`0` (0.0 0.0 0.0) :`1` (`self.GetLaunchLeftVector`) :`2` (`self.GetLaunchRightVector`)) "None" true))
    (:`3`
      (`PrimitiveComponent.AddImpulse` (`/Game/Gameplay/BP_ItemSpawner.Sphere` (`local.ItemSpawner`)) (select `int` CurrentItemIndex :`0` (0.0 0.0 0.0) :`1` (`self.GetLaunchForwardVector`) :`2` (`self.GetLaunchLeftVector`) :`3` (`self.GetLaunchRightVector`)) "None" true))))

(fn `UserConstructionScript`)