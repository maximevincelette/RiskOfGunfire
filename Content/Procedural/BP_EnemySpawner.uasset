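; BP_EnemySpawner is a procedural-generation spawn point that creates one enemy at its own transform whenever SpawnEnemy is called.
; A mode selector picks the class from the passed-in shared types, the spawner's own chosen type, or the calling room's random pick.
; It prints the class name, always spawns despite collisions, and adds BP_Enemy results to the last spawned room's list, not explicitly the calling room's.
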(fn `SpawnEnemy`
  (params (`Calling Room` :type "/Game/Procedural/BP_SpawnableRoom Object Reference") (`All Enemies Same Type - Chosen` :type "/Game/Enemies/BP_Enemy Class Reference") (`All Enemies Same Type -Random` :type "/Game/Enemies/BP_Enemy Class Reference") (SingleOrMultipleEnemyTypes :type "/Game/Core/E_RoomEnemyType Enum" :default "NewEnumerator0"))
  (bind _returnvalue (select `/Game/Core/E_RoomEnemyType` SingleOrMultipleEnemyTypes :`NewEnumerator0` `All Enemies Same Type - Chosen` :`NewEnumerator2` `All Enemies Same Type -Random` :`NewEnumerator3` (`self.All Enemies Different Type - Chosen`) :`NewEnumerator1` (`/Game/Procedural/BP_SpawnableRoom.GetRandomEnemyClass` `Calling Room`) :!type "Actor Class Reference"))
  (`KismetSystemLibrary.PrintString` (`KismetSystemLibrary.GetClassDisplayName` _returnvalue) true true (struct :`R` 0.238418 :`B` 1.0 :`A` 1.0))
  (bind _returnvalue_2 (`|SpawnActorFromClass` _returnvalue (`self.GetTransform`) "AlwaysSpawn" "OverrideRootScale" null null))
  (bind _asbp_enemy (cast `/Game/Enemies/BP_Enemy` _returnvalue_2))
  (`KismetArrayLibrary.Array_Add` (`/Game/Procedural/BP_SpawnableRoom.SpawnedEnemies` (`/Game/Core/BPFL_MainLibrary.GetLastSpawnedRoom`)) _asbp_enemy))

(fn `UserConstructionScript`)