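; BP_Door is a door for procedural room generation that spawns the next random room when the player approaches.
; On BeginPlay it picks a room class from the main game mode's list and unlocks itself if it is the first door.
; Once unlocked, the first player overlap spawns that room at the door's transform, triggering its construction and exit-door spawn.
; Interacting with an unlocked door slides it open once.
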(event `self.ReceiveBeginPlay`
  (set `self.RandomRoomToSpawn` (`self.GetRandomRoom`))
  (if (`self.bIsFirstDoor`)
    (`self.UnlockDoor`)))

(event `/Game/FirstPerson/Blueprints/BPI_Interact.Interact`
  (if (`self.bIsUnlocked`)
    (`/Engine/EditorBlueprintResources/StandardMacros.DoOnce` false
      (:`Completed`
        (`self.OpenDoor`)))))

(event `self.Collision.OnComponentBeginOverlap`
  (params (OverlappedComponent :type "PrimitiveComponent Object Reference") (OtherActor :type "Actor Object Reference") (OtherComp :type "PrimitiveComponent Object Reference") (OtherBodyIndex :type Integer) (bFromSweep :type Boolean) (SweepResult :type "HitResult Structure (by ref)"))
  (cast `/Game/FirstPerson/Blueprints/BP_FirstPersonCharacter` OtherActor)
  (if (`self.bIsUnlocked`)
    (`/Engine/EditorBlueprintResources/StandardMacros.DoOnce` false
      (:`Completed`
        (`self.SpawnRandomRoom`)))))

(fn `CloseDoor`
  (`SceneComponent.K2_AddLocalOffset` (`self.Door_Moving`) (-140.0 0.0 0.0) false false))

(fn `GetRandomRoom`
  (returns (RandomRoomClass :type "/Game/Procedural/BP_SpawnableRoom Class Reference"))
  (return (`KismetArrayLibrary.Array_Random` (`/Game/Core/BP_CustomGameMode.Rooms Classes` (`/Game/Core/BPFL_MainLibrary.Get Main Game Mode`)))))

(fn `OpenDoor`
  (`SceneComponent.K2_AddLocalOffset` (`self.Door_Moving`) (140.0 0.0 0.0) false false))

(fn `SpawnRandomRoom`
  (bind _returnvalue (`|SpawnActorFromClass` (`self.RandomRoomToSpawn`) (`KismetMathLibrary.MakeTransform` (0.0 0.0 0.0) (`self.K2_GetActorRotation`)) "Undefined" "OverrideRootScale" null null))
  (bind _output_get (set `self.SpawnedRoomRef` _returnvalue))
  (`SceneComponent.K2_SetWorldLocation` (`Actor.RootComponent` _output_get) (`self.K2_GetActorLocation`) false true)
  (`/Game/Procedural/BP_SpawnableRoom.StartRoomConstruction` _output_get)
  (`/Game/Procedural/BP_SpawnableRoom.SpawnDoorAtExitPoint` _output_get))

(fn `UnlockDoor`
  (set `self.bIsUnlocked` true)
  (`PrimitiveComponent.SetCollisionProfileName` (`self.Collision`) "OverlapAllDynamic" true))

(fn `UserConstructionScript`)