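; Ammo pickup actor that restores ammo of its AmmoClass type to the first-person player.
; A box overlap casts to BP_FirstPersonCharacter, calls RestoreAmmo once through a DoOnce, then destroys the drop.
; BeginPlay prints the ammo class on screen.
; SetMesh would pick a mesh per weapon class, but it is not wired to run and its mesh options are empty.
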(event `self.ReceiveBeginPlay`
  (`KismetSystemLibrary.PrintString` (`|GetEnumeratorNameAsString` (`self.AmmoClass`)) true true (struct :`R` 1.0 :`B` 0.646856 :`A` 1.0)))

(event `self.Box.OnComponentBeginOverlap`
  (params (OverlappedComponent :type "PrimitiveComponent Object Reference") (OtherActor :type "Actor Object Reference") (OtherComp :type "PrimitiveComponent Object Reference") (OtherBodyIndex :type Integer) (bFromSweep :type Boolean) (SweepResult :type "HitResult Structure (by ref)"))
  (bind _asbp_first_person_character (cast `/Game/Core/BP_FirstPersonCharacter` OtherActor))
  (`/Engine/EditorBlueprintResources/StandardMacros.DoOnce` false
    (:`Completed`
      (`/Game/Core/BP_FirstPersonCharacter.RestoreAmmo` _asbp_first_person_character (`self.AmmoClass`))
      (`self.K2_DestroyActor`))))

(fn `SetMesh`
  (`StaticMeshComponent.SetStaticMesh` (`self.StaticMesh`) (select `/Game/Core/E_WeaponClass` (`self.AmmoClass`) :!type "StaticMesh Object Reference")))

(fn `UserConstructionScript`)