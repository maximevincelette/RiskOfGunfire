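; Base weapon Blueprint that the first-person player can pick up by interacting and later drop.
; Interacting passes the weapon to the character's PickUpWeapon and sets its state to on-player.
; SetGunState toggles mesh physics, collision profiles and info panel visibility between the dropped and carried states, starting as dropped.
; Drop detaches the weapon, restores the dropped state, throws it along the camera's forward vector and removes it from CarriedWeapons.
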(event `self.ReceiveBeginPlay`
  (`parent.ReceiveBeginPlay`)
  (`self.SetGunState` "NewEnumerator0"))

(event `self.ReceiveTick`
  (params (DeltaSeconds :type "Float (single-precision)"))
  (`parent.ReceiveTick` DeltaSeconds))

(event `/Game/Core/BPI_Interact.OnInteracted`
  (params (Player :type "/Game/Core/BP_FirstPersonCharacter Object Reference"))
  (`parent.OnInteracted` null)
  (`self.PickUpGun`)
  (`self.SetGunState` "NewEnumerator1"))

(fn `Drop`
  (params (PlayerRef :type "/Game/Core/BP_FirstPersonCharacter Object Reference"))
  (bind _carriedweapons (`/Game/Core/BP_FirstPersonCharacter.CarriedWeapons` PlayerRef))
  (`self.K2_DetachFromActor` "KeepWorld" "KeepWorld" "KeepWorld")
  (`self.SetGunState` "NewEnumerator0")
  (`PrimitiveComponent.AddImpulse` (`self.SkeletalMesh`) (* (`SceneComponent.GetForwardVector` (`/Game/Core/BP_FirstPersonCharacter.FirstPersonCamera` PlayerRef)) 300.0) "None" true)
  (`KismetArrayLibrary.Array_Remove` _carriedweapons (`KismetArrayLibrary.Array_Find` _carriedweapons self)))

(fn `PickUpGun`
  (bind _asbp_first_person_character (cast `/Game/Core/BP_FirstPersonCharacter` (`GameplayStatics.GetPlayerCharacter` 0)))
  (`/Game/Core/BP_FirstPersonCharacter.PickUpWeapon` _asbp_first_person_character self))

(fn `SetGunState`
  (params (NewWeaponState :type "/Game/Core/EWeaponState Enum" :default "NewEnumerator0"))
  (bind _output_get (set `self.Weapon State` NewWeaponState))
  (switch `/Game/Core/EWeaponState` _output_get
    (:`NewEnumerator0`
      (`PrimitiveComponent.SetCollisionProfileName` (`self.SkeletalMesh`) "DroppedWeapon" true)
      (`PrimitiveComponent.SetCollisionProfileName` (`self.InteractCollision`) "IgnoreAllExceptTraces" true)
      (`PrimitiveComponent.SetSimulatePhysics` (`self.SkeletalMesh`) true)
      (bind _iteminfopannel (`self.ItemInfoPannel`)
        (:`then`
          (`PrimitiveComponent.SetCollisionProfileName` _iteminfopannel "IgnoreAllExceptTraces" true)
          (`SceneComponent.SetVisibility` _iteminfopannel true false))
        (:`else`)))
    (:`NewEnumerator1`
      (`PrimitiveComponent.SetSimulatePhysics` (`self.SkeletalMesh`) false)
      (`PrimitiveComponent.SetCollisionProfileName` (`self.InteractCollision`) "NoCollision" true)
      (`PrimitiveComponent.SetCollisionProfileName` (`self.SkeletalMesh`) "NoCollision" true)
      (`PrimitiveComponent.SetCollisionResponseToChannel` (`self.InteractCollision`) "ECC_GameTraceChannel2" "ECR_Ignore")
      (`PrimitiveComponent.SetCollisionResponseToChannel` (`self.SkeletalMesh`) "ECC_GameTraceChannel2" "ECR_Ignore")
      (`PrimitiveComponent.SetCollisionResponseToChannel` (`self.InteractCollision`) "ECC_Visibility" "ECR_Ignore")
      (`PrimitiveComponent.SetCollisionResponseToChannel` (`self.SkeletalMesh`) "ECC_Visibility" "ECR_Ignore")
      (`PrimitiveComponent.SetCollisionProfileName` (`self.SkeletalMesh`) "NoCollision" true)
      (bind _iteminfopannel_2 (`self.ItemInfoPannel`)
        (:`then`
          (`PrimitiveComponent.SetCollisionResponseToAllChannels` _iteminfopannel_2 "ECR_Ignore")
          (`SceneComponent.SetVisibility` _iteminfopannel_2 false false))
        (:`else`)))))

(fn `UserConstructionScript`
  (`parent.UserConstructionScript`))