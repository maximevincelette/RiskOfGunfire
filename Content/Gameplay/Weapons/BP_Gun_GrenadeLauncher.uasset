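; Grenade launcher weapon Blueprint that fires one physics-driven grenade projectile each time shooting starts, while ammo remains.
; It extends a parent gun class and expects its parent actor to be the first-person character.
; FireBullet spawns a scaled-down grenade at the barrel reference point, oriented by the player camera or, with alternate firing, the barrel.
; It then launches the grenade's sphere with a forward impulse scaled by bullet speed and decrements ammo.
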(event `self.ReceiveTick`
  (params (DeltaSeconds :type "Float (single-precision)"))
  (`parent.ReceiveTick` DeltaSeconds))

(event `self.StartShooting`
  (`parent.StartShooting`)
  (`self.FireBullet`))

(event `self.StopShooting`
  (`parent.StopShooting`))

(fn `FireBullet`
  (bind _asbp_first_person_character (cast `/Game/Core/BP_FirstPersonCharacter` (`self.GetParentActor`)))
  (if (> (`self.AmmoCount_0`) 0)
    (if (`self.bAlternateFiring_0`)
      (set `self.Direction_0` (`SceneComponent.K2_GetComponentRotation` (`self.Barrel_RefPoint_0`)))
      (else
        (set `self.Direction_0` (`SceneComponent.K2_GetComponentRotation` (`/Game/Core/BP_FirstPersonCharacter.FirstPersonCamera` _asbp_first_person_character)))))
    (bind _returnvalue (`|SpawnActorFromClass` "/Game/Gameplay/Weapons/Projectiles/BP_Projectile_Grenade.BP_Projectile_Grenade_C" (`KismetMathLibrary.MakeTransform` (`SceneComponent.K2_GetComponentLocation` (`self.Barrel_RefPoint_0`)) (`self.Direction_0`) (0.1 0.1 0.1)) "Undefined" "OverrideRootScale" null null))
    (`PrimitiveComponent.AddImpulse` (`/Game/Gameplay/Weapons/Projectiles/BP_Projectile_Grenade.Sphere` _returnvalue) (* (`KismetMathLibrary.Normal` (`KismetMathLibrary.GetForwardVector` (`self.Direction_0`))) (`self.BulletSpeed_0`)) "None" false)
    (`/Engine/EditorBlueprintResources/StandardMacros.DecrementInt` (`self.AmmoCount_0`))))

(fn `UserConstructionScript`
  (`parent.UserConstructionScript`))