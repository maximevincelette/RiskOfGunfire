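; Base gun Blueprint that handles firing modes, alternate-fire state and reloading, leaving FireBullet empty.
; StartShooting branches on FiringMode: semi-automatic uses a delay, fully automatic a looping timer cleared by StopShooting, and burst a DoN loop with delays between shots and bursts.
; ReloadGun starts a timer if CanReload passes, then UpdateAmmoCount refills the magazine from reserve ammo.
; Tick tracks reload progress as a fraction of reload time.
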(event `self.ReceiveTick`
  (params (DeltaSeconds :type "Float (single-precision)"))
  (if (`self.bReloading`)
    (set `self.ReloadTimerPercentage` (/ (`KismetSystemLibrary.K2_GetTimerElapsedTimeHandle` (`self.ReloadTimer`)) (`self.ReloadingTime`)))))

(event `StartShooting`
  (if (and (not (`self.bReloading`)) (not (`self.bFiring`)))
    (set `self.bFiring` true)
    (switch `/Game/Core/EFiringMode` (`self.FiringMode`)
      (:`NewEnumerator0`
        (`self.FireBullet`)
        (`KismetSystemLibrary.Delay` (/ 60.0 (`self.SemiAutomatic_FireRate_RPM`)))
        (set `self.bFiring` false))
      (:`NewEnumerator1`
        (`self.FireBullet`)
        (bind _returnvalue (`KismetSystemLibrary.K2_SetTimer` null "FireBullet" (/ 60.0 (`self.FullyAutomatic_FireRate_RPM`)) true))
        (set `self.AutomaticGunTimer` _returnvalue))
      (:`NewEnumerator2`
        (if (not (`self.bFiringBurst`))
          (bind _counter (`/Engine/EditorBlueprintResources/StandardMacros.Do N` (`self.ShotsPerBurst`) :!label _label)
            (:`Exit`
              (set `self.bFiringBurst` true)
              (`self.FireBullet`)
              (`KismetSystemLibrary.Delay` (/ 60.0 (`self.BurstFireRate`)))
              (if (not (== _counter (`self.ShotsPerBurst`)))
                (goto _label)
                (else
                  (set `self.bFiring` false)
                  (`KismetSystemLibrary.Delay` (`self.BetweenBurstDelay`))
                  (set `self.bFiringBurst` false)
                  (`self.ResetBurst`))))))))))

(event `StopShooting`
  (switch `/Game/Core/EFiringMode` (`self.FiringMode`)
    (:`NewEnumerator1`
      (set `self.bFiring` false)
      (`KismetSystemLibrary.K2_ClearAndInvalidateTimerHandle` (`self.AutomaticGunTimer`)))
    (:`NewEnumerator2`
      (set `self.bFiring` false))))

(event `ResetBurst`
  (goto _label :!via `Reset`))

(event `StartAlternateFire`
  (set `self.bAlternateFiring` true))

(event `StopAlternateFire`
  (set `self.bAlternateFiring` false))

(event `ReloadGun`
  (if (`self.CanReload`)
    (bind _returnvalue (`KismetSystemLibrary.K2_SetTimer` null "UpdateAmmoCount" (`self.ReloadingTime`)))
    (set `self.ReloadTimer` _returnvalue)
    (set `self.bReloading` true)))

(fn `CanReload`
  (returns (ReturnValue :type Boolean))
  (return (and (!= (`self.AmmoCount`) (`self.MagSize`)) (!= (`self.AmmoMax`) 0) (not (`self.bReloading`)))))

(fn `FireBullet`)

(fn `UpdateAmmoCount`
  (bind _output_get (set `self.BulletDifference` (- (`self.MagSize`) (`self.AmmoCount`))))
  (if (>= (`self.AmmoMax`) _output_get)
    (set `self.AmmoCount` (`self.MagSize`))
    (set `self.AmmoMax` (- (`self.AmmoMax`) (`self.BulletDifference`)))
    (else
      (set `self.AmmoCount` (+ (`self.AmmoCount`) (`self.AmmoMax`)))
      (set `self.AmmoMax` 0)))
  (set `self.bReloading` false))

(fn `UserConstructionScript`
  (`parent.UserConstructionScript`))