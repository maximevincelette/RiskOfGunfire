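; Parent Blueprint for projectile-based guns, implementing bullet firing by spawning projectile actors.
; FireBullet requires the gun to have ammo and not be reloading, then spawns the configured projectile class at the barrel reference point.
; Shots follow the player's first-person camera rotation, or the barrel's own rotation during alternate firing.
; Each projectile receives scale, speed and final damage, then the gun debug-prints the damage and decrements ammo.
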(fn `FireBullet`
  (bind _finaldamage (`self.FinalDamage`))
  (if (not (`self.bReloading`))
    (bind _asbp_first_person_character (cast `/Game/Core/BP_FirstPersonCharacter` (`GameplayStatics.GetPlayerCharacter` 0)))
    (if (> (`self.CurrentAmmoCount`) 0)
      (if (`self.bAlternateFiring`)
        (set `self.Direction` (`SceneComponent.K2_GetComponentRotation` (`self.Barrel_RefPoint`)))
        (else
          (set `self.Direction` (`SceneComponent.K2_GetComponentRotation` (`/Game/Core/BP_FirstPersonCharacter.FirstPersonCamera` _asbp_first_person_character)))))
      (`|SpawnActorFromClass` (`self.Projectile Class`) (`KismetMathLibrary.MakeTransform` (`SceneComponent.K2_GetComponentLocation` (`self.Barrel_RefPoint`)) (`self.Direction`) (`KismetMathLibrary.Conv_DoubleToVector` (`self.Projectile Scale`))) "Undefined" "OverrideRootScale" null (`self.Bullet Speed`) _finaldamage null)
      (`KismetSystemLibrary.PrintString` (`KismetStringLibrary.Conv_DoubleToString` _finaldamage) true true (struct :`R` 0.236625 :`B` 1.0 :`A` 1.0) 5.0)
      (`/Engine/EditorBlueprintResources/StandardMacros.DecrementInt` (`self.CurrentAmmoCount`)))))

(fn `UserConstructionScript`
  (`parent.UserConstructionScript`))