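; Grenade launcher weapon Blueprint that inherits its shooting behavior from a parent class, likely a projectile gun base.
; BeginPlay calls the parent, then casts and caches the first-person player character.
; Tick, StartShooting, StopShooting and the construction script only forward to the parent.
; An unconnected debug print compares base and final damage using the character's damage-type multiplier, but never runs.
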(event `self.ReceiveBeginPlay`
  (`parent.ReceiveBeginPlay`)
  (bind _asbp_first_person_character (cast `/Game/Core/BP_FirstPersonCharacter` (`GameplayStatics.GetPlayerCharacter` 0)))
  (set `self.As BP First Person Character` _asbp_first_person_character))

(event `self.ReceiveTick`
  (params (DeltaSeconds :type "Float (single-precision)"))
  (`parent.ReceiveTick` DeltaSeconds))

(event `self.StartShooting`
  (`parent.StartShooting`))

(event `self.StopShooting`
  (`parent.StopShooting`))

(fn `UserConstructionScript`
  (`parent.UserConstructionScript`))