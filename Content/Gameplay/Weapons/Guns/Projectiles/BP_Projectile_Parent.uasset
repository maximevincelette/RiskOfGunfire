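; Base projectile Blueprint for guns, with a capsule for overlap detection and a projectile movement component.
; When the movement component activates, it copies the ProjectileSpeed variable into both initial and max speed and prints the value.
; Capsule overlaps only print a "Hit" debug message, with no damage or destroy logic.
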(event `self.ReceiveBeginPlay`)

(event `self.Capsule.OnComponentBeginOverlap`
  (params (OverlappedComponent :type "PrimitiveComponent Object Reference") (OtherActor :type "Actor Object Reference") (OtherComp :type "PrimitiveComponent Object Reference") (OtherBodyIndex :type Integer) (bFromSweep :type Boolean) (SweepResult :type "HitResult Structure (by ref)"))
  (`KismetSystemLibrary.PrintString` "Hit" true true (struct :`R` 1.0 :`G` 0.176017 :`A` 1.0)))

(event `self.ProjectileMovement.OnComponentActivated`
  (params (Component :type "ActorComponent Object Reference") (bReset :type Boolean))
  (set `ProjectileMovementComponent.InitialSpeed` (`self.ProjectileSpeed`) (`self.ProjectileMovement`))
  (set `ProjectileMovementComponent.MaxSpeed` (`self.ProjectileSpeed`) (`self.ProjectileMovement`))
  (`KismetSystemLibrary.PrintString` (`KismetStringLibrary.Conv_DoubleToString` (`self.ProjectileSpeed`)) true true (struct :`R` 1.0 :`B` 0.007519 :`A` 1.0)))

(fn `UserConstructionScript`)