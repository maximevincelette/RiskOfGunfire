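; Bouncing grenade projectile that explodes on contact with an enemy or shortly after bouncing off anything else.
; The projectile movement bounce event casts the hit actor to BP_Enemy_Parent, calling Explode immediately on success or after BounceExplosionDelay otherwise.
; Explode is not defined in this graph.
; BeginPlay runs the parent logic, then prints ProjectileDamage on screen as debug output.
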(event `self.ReceiveBeginPlay`
  (`parent.ReceiveBeginPlay`)
  (`KismetSystemLibrary.PrintString` (`KismetStringLibrary.Conv_DoubleToString` (`self.ProjectileDamage`)) true true (struct :`G` 1.0 :`B` 0.703727 :`A` 1.0) 3.0))

(event `self.ProjectileMovement.OnProjectileBounce`
  (params (ImpactResult :type "HitResult Structure (by ref)") (ImpactVelocity :type "Vector Structure (by ref)"))
  (cast `/Game/Gameplay/Enemies/BP_Enemy_Parent` ImpactResult_HitActor
    (:`then`
      (`self.Explode`))
    (:`CastFailed`
      (`KismetSystemLibrary.Delay` (`self.BounceExplosionDelay`))
      (`self.Explode`))))

(fn `UserConstructionScript`
  (`parent.UserConstructionScript`))