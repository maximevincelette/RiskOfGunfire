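; Shotgun hitscan weapon that spends one round to fire several pellets from the player's first-person camera.
; FireBullet, gated by reload state and ammo, runs a multi sphere trace per pellet toward a random point in a cone cross-section sized by BulletAngle and Range.
; Non-blocking hits damage BP_Enemy_Parent actors, while blocking hits only print debug text.
; Random angle and linear radius sampling clusters pellets toward the center.
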(event `self.ReceiveBeginPlay`
  (`parent.ReceiveBeginPlay`)
  (set `self.BulletAngle` (`self.StartingBulletAngle`)))

(fn `FireBullet`
  (bind _firstpersoncamera (`/Game/Core/BP_FirstPersonCharacter.FirstPersonCamera` (`self.PlayerRef`)))
  (bind _returnvalue (`SceneComponent.GetForwardVector` _firstpersoncamera))
  (bind _returnvalue_2 (+ (`SceneComponent.K2_GetComponentLocation` _firstpersoncamera) (* (`KismetMathLibrary.Normal` _returnvalue) 100.0)))
  (if (not (`self.bReloading`))
    (if (> (`self.CurrentAmmoCount`) 0)
      (`/Engine/EditorBlueprintResources/StandardMacros.DecrementInt` (`self.CurrentAmmoCount`)
        (:`  `
          (for _ (range (`self.PelletsAmount`))
            (bind _point (`self.GetRandomPointInCircle` (* (`KismetMathLibrary.DegTan` (`self.BulletAngle`)) (`self.Range`))))
            (bind (_x _y) (`KismetMathLibrary.BreakVector2D` _point))
            (bind _outhits (`KismetSystemLibrary.SphereTraceMulti` :`Start` _returnvalue_2 :`End` (+ (+ _returnvalue_2 (* _returnvalue (`self.Range`))) (* (`SceneComponent.GetRightVector` _firstpersoncamera) _x) (* (`SceneComponent.GetUpVector` _firstpersoncamera) _y)) :`Radius` (`self.SphereTraceRadius`) :`TraceChannel` "TraceTypeQuery3" :`TraceColor` (struct :`R` 1.0 :`G` 0.384752 :`A` 1.0) :`TraceHitColor` (struct :`G` 0.567708 :`B` 0.041446 :`A` 1.0)))
            (for _array_element _outhits
              (bind (_bblockinghit _binitialoverlap _time _distance _location _impactpoint _normal _impactnormal _physmat _hitactor _hitcomponent) (`GameplayStatics.BreakHitResult` _array_element))
              (if (not _bblockinghit)
                (set `self.Impact Point` _impactpoint)
                (bind _asbp_enemy_parent (cast `/Game/Gameplay/Enemies/BP_Enemy_Parent` _hitactor))
                (`GameplayStatics.ApplyDamage` _asbp_enemy_parent (`self.FinalDamage`))
                (set `self.LastHitActor` _hitactor)
                (else
                  (`KismetSystemLibrary.PrintText` (`|FormatText` "Blocking Hit \nActor : {x} \nComponent : {y}" _hitactor _hitcomponent) true true (struct :`R` 1.0 :`G` 0.437199 :`A` 1.0) 3.0))))))))))

(fn `GetRandomPointInCircle`
  (params (Radius :type "Float (double-precision)"))
  (returns (Point :type "Vector2D Structure"))
  (locals (Angle :type "Float (double-precision)") (DistanceFromCenter :type "Float (double-precision)"))
  (set `local.Angle` (`KismetMathLibrary.RandomFloatInRange` 0.0 360.0))
  (set `local.DistanceFromCenter` (`KismetMathLibrary.RandomFloatInRange` 0.0 (`local.Radius`)))
  (return (`KismetMathLibrary.MakeVector2D` (* (`local.DistanceFromCenter`) (`KismetMathLibrary.DegCos` (`local.Angle`))) (* (`local.DistanceFromCenter`) (`KismetMathLibrary.DegSin` (`local.Angle`))))))

(fn `UserConstructionScript`
  (`parent.UserConstructionScript`))