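; Hitscan electric arc gun whose shot chains damage between nearby enemies.
; After the parent fires, FireBullet starts at the last hit actor and repeatedly finds the closest BP_Enemy_Parent, ignoring those already hit.
; Each one within ArcBounceRange takes the full FinalDamage and becomes the next arc origin, with no cap on bounce count.
; The chain only applies damage and prints debug text; it spawns no arc visuals.
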(fn `FireBullet`
  (bind _alreadyhitenemies (`self.AlreadyHitEnemies`))
  (`parent.FireBullet`)
  (`KismetArrayLibrary.Array_Clear` _alreadyhitenemies)
  (`KismetArrayLibrary.Array_Add` _alreadyhitenemies (`self.LastHitActor`))
  (bind _output_get (set `self.ArcOriginActor` (`self.LastHitActor`)))
  (`/Engine/EditorBlueprintResources/StandardMacros.IsValid` _output_get :!label _label
    (:`Is Valid`
      (set `self.ArcOriginLocation` (`self.K2_GetActorLocation` _output_get)))
    (:`Is Not Valid`
      _))
  (bind (_closestactor _closestactordistance) (`/Game/Core/BPFL_MainLibrary.GetClosestActorOfClass` "/Game/Gameplay/Enemies/BP_Enemy_Parent.BP_Enemy_Parent_C" (`self.ArcOriginLocation`) (`self.AlreadyHitEnemies`)))
  (if (not (`KismetArrayLibrary.Array_Contains` (`self.AlreadyHitEnemies`) _closestactor))
    (`KismetSystemLibrary.PrintText` (`|FormatText` "Closest Actor : {x} \nDistance : {y}" _closestactor _closestactordistance) true true (struct :`R` 0.589812 :`G` 0.259244 :`B` 1.0 :`A` 1.0) 3.0)
    (if (<= _closestactordistance (`self.ArcBounceRange`))
      (bind _output_get_2 (set `self.ArcOriginActor` _closestactor))
      (set `self.ArcOriginLocation` (`self.K2_GetActorLocation` _output_get_2))
      (`KismetArrayLibrary.Array_Add` (`self.AlreadyHitEnemies`) _output_get_2)
      (bind _asbp_enemy_parent (cast `/Game/Gameplay/Enemies/BP_Enemy_Parent` _output_get_2))
      (`GameplayStatics.ApplyDamage` _asbp_enemy_parent (`self.FinalDamage`))
      (goto _label))))

(fn `UserConstructionScript`
  (`parent.UserConstructionScript`))