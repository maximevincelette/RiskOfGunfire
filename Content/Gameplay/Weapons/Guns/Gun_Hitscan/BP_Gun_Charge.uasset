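; BP_Gun_Charge is a charge-up gun Blueprint that builds charge while shooting is held and fires on release.
; StartShooting plays the ChargeWeapon timeline when no charge remains, writing its clamped value to CurrentCharge and calling StopShooting automatically at full charge.
; StopShooting calls FireBullet once the charge reaches MinimumChargeToShoot, then reverses the timeline to drain the charge.
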(event `self.StartShooting`
  (`parent.StartShooting`)
  (if (and (not (`self.bCharging`)) (<= (`self.CurrentCharge`) 0.0))
    (set `self.bCharging` true)
    (bind (_direction _weaponcharge) (`Timeline|ChargeWeapon` :!label _label)
      (:`Update`
        (bind _output_get (set `self.CurrentCharge` (`KismetMathLibrary.FClamp` _weaponcharge)))
        (if (>= _output_get 1.0)
          (`self.StopShooting`))))))

(event `self.StopShooting`
  (`parent.StopShooting`)
  (if (and (`self.bCharging`) (>= (`self.CurrentCharge`) (`self.MinimumChargeToShoot`)))
    (`self.FireBullet`)
    (goto _label :!via `Reverse`)))

(fn `UserConstructionScript`
  (`parent.UserConstructionScript`))