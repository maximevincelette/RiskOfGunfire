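; Base hitscan gun that fires a shot when shooting starts, extending its parent gun's shoot and alternate-fire events.
; FireBullet skips while reloading or empty, otherwise spends one round on a multi sphere trace from just ahead of the first-person camera, with debug drawing on.
; Non-blocking hits let shots pierce: enemies within the per-shot hit limit receive a damage call and are destroyed outright, until a blocking hit ends the loop.
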(event `self.StartShooting`
  (`parent.StartShooting`)
  (`self.FireBullet`))

(event `self.StopShooting`
  (`parent.StopShooting`))

(event `self.StartAlternateFire`
  (`parent.StartAlternateFire`))

(event `self.StopAlternateFire`
  (`parent.StopAlternateFire`))

(fn `FireBullet`
  (if (not (`self.bReloading`))
    (bind _asbp_first_person_character (cast `/Game/Core/BP_FirstPersonCharacter` (`self.GetParentActor`)))
    (if (> (`self.AmmoCount`) 0)
      (bind _firstpersoncamera (`/Game/Core/BP_FirstPersonCharacter.FirstPersonCamera` _asbp_first_person_character))
      (bind (_tracestart _traceend) (`/Game/Core/BPFL_MainLibrary.Get Trace Vectors` "NewEnumerator0" (`self.Range`) self true _firstpersoncamera (+ (`SceneComponent.K2_GetComponentLocation` _firstpersoncamera) (* (`KismetMathLibrary.Normal` (`SceneComponent.GetForwardVector` _firstpersoncamera)) 100.0))))
      (bind _outhits (`KismetSystemLibrary.SphereTraceMulti` :`Start` _tracestart :`End` _traceend :`Radius` (`self.SphereTraceRadius`) :`TraceChannel` "TraceTypeQuery1" :`DrawDebugType` "ForDuration" :`TraceColor` (struct :`R` 1.0 :`G` 0.384752 :`A` 1.0) :`TraceHitColor` (struct :`G` 0.567708 :`B` 0.041446 :`A` 1.0)))
      (`/Engine/EditorBlueprintResources/StandardMacros.DecrementInt` (`self.AmmoCount`)
        (:`  `
          (for (_array_element _array_index) _outhits
            (bind (_bblockinghit _binitialoverlap _time _distance _location _impactpoint _normal _impactnormal _physmat _hitactor) (`GameplayStatics.BreakHitResult` _array_element))
            (if (not _bblockinghit)
              (if (<= _array_index (- (`self.MaxEnemiesHitPerShot`) 1))
                (bind _asbp_enemy (cast `/Game/Enemies/BP_Enemy` _hitactor))
                (`GameplayStatics.ApplyDamage` _asbp_enemy)
                (`self.K2_DestroyActor` _asbp_enemy))
              (else
                (break)))))))))

(fn `UserConstructionScript`
  (`parent.UserConstructionScript`))