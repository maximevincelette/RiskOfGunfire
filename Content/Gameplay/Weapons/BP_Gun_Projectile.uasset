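; BP_Gun_Projectile is a gun that fires physical projectiles for its parent BP_FirstPersonCharacter.
; FireBullet, blocked while reloading or out of ammo, spawns a scaled-down BP_FirstPersonProjectile at the barrel reference point and decrements the ammo count.
; Shots follow the character's camera rotation, or the barrel's own rotation when AlternateFiring is set.
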(fn `FireBullet`
  (if (not (`self.bReloading`))
    (bind _asbp_first_person_character (cast `/Game/Core/BP_FirstPersonCharacter` (`self.GetParentActor`)))
    (if (> (`self.AmmoCount`) 0)
      (if (`self.bAlternateFiring`)
        (set `self.Direction` (`SceneComponent.K2_GetComponentRotation` (`self.Barrel_RefPoint`)))
        (else
          (set `self.Direction` (`SceneComponent.K2_GetComponentRotation` (`/Game/Core/BP_FirstPersonCharacter.FirstPersonCamera` _asbp_first_person_character)))))
      (`|SpawnActorFromClass` "/Game/FirstPerson/Blueprints/BP_FirstPersonProjectile.BP_FirstPersonProjectile_C" (`KismetMathLibrary.MakeTransform` (`SceneComponent.K2_GetComponentLocation` (`self.Barrel_RefPoint`)) (`self.Direction`) (0.1 0.1 0.1)) "Undefined" "OverrideRootScale" null null)
      (`/Engine/EditorBlueprintResources/StandardMacros.DecrementInt` (`self.AmmoCount`)))))

(fn `UserConstructionScript`
  (`parent.UserConstructionScript`))