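; Full-auto gun Blueprint that extends a parent weapon with continuous fire and an aim view as alternate fire.
; Shooting fires at once, then a looping timer calls FireBullet at an interval derived from FireRateRPM until stopped.
; Alternate fire blends the player's view to the gun and back to its parent actor.
; While it is active, Tick keeps the first-person character's camera aligned with control rotation.
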(event `self.StartShooting`
  (`parent.StartShooting`)
  (`self.FireBullet`)
  (bind _returnvalue (`KismetSystemLibrary.K2_SetTimer` null "FireBullet" (/ 60.0 (`self.FireRateRPM`)) true))
  (set `self.GunTimer` _returnvalue))

(event `self.StopShooting`
  (`parent.StopShooting`)
  (`KismetSystemLibrary.K2_ClearAndInvalidateTimerHandle` (`self.GunTimer`)))

(event `self.StartAlternateFire`
  (`parent.StartAlternateFire`)
  (`PlayerController.SetViewTargetWithBlend` (`GameplayStatics.GetPlayerController` 0) self 0.2 "VTBlend_Linear" 0.0 false))

(event `self.StopAlternateFire`
  (`parent.StopAlternateFire`)
  (`PlayerController.SetViewTargetWithBlend` (`GameplayStatics.GetPlayerController` 0) (`self.GetParentActor`) 0.2 "VTBlend_Linear" 0.0 false))

(event `self.ReceiveTick`
  (params (DeltaSeconds :type "Float (single-precision)"))
  (`parent.ReceiveTick` 0.0)
  (if (`self.bAlternateFiring`)
    (bind _asbp_first_person_character (cast `/Game/Core/BP_FirstPersonCharacter` (`GameplayStatics.GetPlayerCharacter` 0)))
    (`SceneComponent.K2_SetWorldRotation` (`/Game/Core/BP_FirstPersonCharacter.FirstPersonCamera` _asbp_first_person_character) (`Controller.GetControlRotation` (`GameplayStatics.GetPlayerController` 0)) false false)))

(fn `UserConstructionScript`
  (`parent.UserConstructionScript`))