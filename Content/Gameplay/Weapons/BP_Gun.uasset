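; BP_Gun is a gun Blueprint that tracks firing, alternate-fire and reload state, with an empty FireBullet function.
; Start and stop events set the fire flags, with primary fire blocked during reloads.
; ReloadGun checks CanReload, then starts a timer that calls UpdateAmmoCount to refill the magazine from reserve ammo.
; Tick updates reload progress from the timer and prints the Reloading flag for debugging.
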(event `self.ReceiveTick`
  (params (DeltaSeconds :type "Float (single-precision)"))
  (`KismetSystemLibrary.PrintString` (`KismetStringLibrary.Conv_BoolToString` (`self.bReloading`)) true true (struct :`R` 1.0 :`G` 0.91148 :`A` 1.0) 0.0)
  (if (`self.bReloading`)
    (set `self.ReloadTimerPercentage` (/ (`KismetSystemLibrary.K2_GetTimerElapsedTimeHandle` (`self.ReloadTimer`)) (`self.ReloadingTime`)))))

(event `StartShooting`
  (if (not (`self.bReloading`))
    (set `self.bFiring` true)))

(event `StopShooting`
  (set `self.bFiring` false))

(event `StartAlternateFire`
  (set `self.bAlternateFiring` true))

(event `StopAlternateFire`
  (set `self.bAlternateFiring` false))

(event `ReloadGun`
  (if (`self.CanReload`)
    (bind _returnvalue (`KismetSystemLibrary.K2_SetTimer` null "UpdateAmmoCount" (`self.ReloadingTime`)))
    (set `self.ReloadTimer` _returnvalue)
    (set `self.bReloading` true)
    (set `self.bFiring` false)))

(fn `CanReload`
  (returns (ReturnValue :type Boolean))
  (return (and (!= (`self.AmmoCount`) (`self.MagSize`)) (!= (`self.AmmoMax`) 0) (not (`self.bReloading`)))))

(fn `FireBullet`)

(fn `UpdateAmmoCount`
  (bind _output_get (set `self.BulletDifference` (- (`self.MagSize`) (`self.AmmoCount`))))
  (if (>= (`self.AmmoMax`) _output_get)
    (set `self.AmmoCount` (`self.MagSize`))
    (set `self.AmmoMax` (- (`self.AmmoMax`) (`self.BulletDifference`)))
    (else
      (set `self.AmmoCount` (+ (`self.AmmoCount`) (`self.AmmoMax`)))
      (set `self.AmmoMax` 0)))
  (set `self.bReloading` false))

(fn `UserConstructionScript`
  (`parent.UserConstructionScript`))