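; BP_Weapon is a pickup laser weapon that snaps to the first-person character's GripPoint socket when that character overlaps its collision sphere.
; On pickup it binds to the character's use and stop-using item events.
; Firing spawns one BP_Laser at the spawn point, aimed by camera rotation with a slight yaw offset, and attaches it there keeping world rotation.
; Stopping fire destroys that laser.
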(event `self.SphereCollision.OnComponentBeginOverlap`
  (params (OverlappedComponent :type "PrimitiveComponent Object Reference") (OtherActor :type "Actor Object Reference") (OtherComp :type "PrimitiveComponent Object Reference") (OtherBodyIndex :type Integer) (bFromSweep :type Boolean) (SweepResult :type "HitResult Structure (by ref)"))
  (bind _asbp_first_person_character (cast `/Game/FirstPerson/Blueprints/BP_FirstPersonCharacter` OtherActor))
  (bind _output_get (set `self.FirstPersonCharacterRef` _asbp_first_person_character))
  (`self.K2_AttachToComponent` self (`/Game/FirstPerson/Blueprints/BP_FirstPersonCharacter.FirstPersonMesh` _output_get) "GripPoint" "SnapToTarget" "SnapToTarget" "SnapToTarget" true)
  (add `/Game/FirstPerson/Blueprints/BP_FirstPersonCharacter.OnUseItem` (`self.FirstPersonCharacterRef`) (`|CreateDelegate` :!event `OnFireProjectile`))
  (add `/Game/FirstPerson/Blueprints/BP_FirstPersonCharacter.OnStopUsingItem` (`self.FirstPersonCharacterRef`) (`|CreateDelegate` :!event `OnStopFiring`)))

(event `OnFireProjectile`
  (bind (_returnvalue_roll _returnvalue_pitch _returnvalue_yaw) (`KismetMathLibrary.BreakRotator` (`PlayerCameraManager.GetCameraRotation` (`GameplayStatics.GetPlayerCameraManager` 0))))
  ;[1 1 1] Fire projectile
  (if (not (`KismetSystemLibrary.IsValid` (`self.LaserInstance`)))
    (bind _returnvalue (`|SpawnActorFromClass` "/Game/Gameplay/BP_Laser.BP_Laser_C" (`KismetMathLibrary.MakeTransform` (`SceneComponent.K2_GetComponentLocation` (`self.SpawnPoint`)) (`KismetMathLibrary.MakeRotator` _returnvalue_roll _returnvalue_pitch (- _returnvalue_yaw 3.0))) "Undefined" "OverrideRootScale" null null))
    (bind _output_get (set `self.LaserInstance` _returnvalue))
    (`self.K2_AttachToComponent` _output_get (`self.SpawnPoint`) "None" "SnapToTarget" "KeepWorld" "KeepWorld" true)))

(event `OnStopFiring`
  (if (`KismetSystemLibrary.IsValid` (`self.LaserInstance`))
    (`self.K2_DestroyActor` (`self.LaserInstance`))))

(fn `UserConstructionScript`)