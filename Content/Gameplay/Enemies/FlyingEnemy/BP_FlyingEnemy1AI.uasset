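; Flying enemy pawn that roams at random and switches on AI behavior when the first-person player comes near.
; Tick uses a random Delay to pace AIMoveTo calls toward random reachable points within Radius.
; Player overlap with Sphere runs BT_FlyingAI; leaving only stops the controller's current movement, without stopping the tree or roam loop.
; The Moving flag is set true before each move and on both success and failure, never cleared.
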(event `self.ReceiveBeginPlay`)

(event `self.ReceiveTick`
  (params (DeltaSeconds :type "Float (single-precision)"))
  ;[1 1 1] AI Random roam
  (`KismetSystemLibrary.Delay` (`KismetMathLibrary.RandomFloatInRange` 1.0 5.0))
  (set `self.bMoving` true)
  (`|AIMoveTo` self (`NavigationSystemV1.K2_GetRandomReachablePointInRadius` (`self.K2_GetActorLocation`) (`self.Radius`) null null) null
    (:`OnSuccess`
      _)
    (:`OnFail`
      _))
  (set `self.bMoving` true))

(event `self.Sphere.OnComponentBeginOverlap`
  (params (OverlappedComponent :type "PrimitiveComponent Object Reference") (OtherActor :type "Actor Object Reference") (OtherComp :type "PrimitiveComponent Object Reference") (OtherBodyIndex :type Integer) (bFromSweep :type Boolean) (SweepResult :type "HitResult Structure (by ref)"))
  (cast `/Game/Core/BP_FirstPersonCharacter` OtherActor)
  (`AIController.RunBehaviorTree` (`AIBlueprintHelperLibrary.GetAIController` self) "/Game/Gameplay/Enemies/FlyingEnemy/BT_FlyingAI.BT_FlyingAI"))

(event `self.Sphere.OnComponentEndOverlap`
  (params (OverlappedComponent :type "PrimitiveComponent Object Reference") (OtherActor :type "Actor Object Reference") (OtherComp :type "PrimitiveComponent Object Reference") (OtherBodyIndex :type Integer))
  (cast `/Game/Core/BP_FirstPersonCharacter` OtherActor)
  (`Controller.StopMovement` (`AIBlueprintHelperLibrary.GetAIController` self)))

(fn `UserConstructionScript`)