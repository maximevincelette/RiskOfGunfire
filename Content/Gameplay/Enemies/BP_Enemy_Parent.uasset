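; Base enemy Blueprint that handles armor, health and death.
; AnyDamage drains armor with percentage reduction, spills excess into health, updates the health bar widget and spawns on-screen damage numbers.
; On death it notifies the last spawned room, may drop ammo for a random weapon the player carries, then destroys itself.
; The health bar turns toward the player each tick; RadialDamage only prints a debug string.
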(event `self.ReceiveTick`
  (params (DeltaSeconds :type "Float (single-precision)"))
  (`self.RotateHealthBar`))

(event `self.ReceiveBeginPlay`
  (`self.InitiateStartValues`)
  (`self.InitiateHealthBar`))

(event `self.ReceiveAnyDamage`
  (params (Damage :type "Float (single-precision)") (DamageType :type "DamageType Object Reference") (InstigatedBy :type "Controller Object Reference") (DamageCauser :type "Actor Object Reference"))
  (`self.CalculateDamage` Damage))

(event `self.ReceiveRadialDamage`
  (params (DamageReceived :type "Float (single-precision)") (DamageType :type "DamageType Object Reference") (Origin :type "Vector Structure") (HitInfo :type "HitResult Structure (by ref)") (InstigatedBy :type "Controller Object Reference") (DamageCauser :type "Actor Object Reference"))
  (`KismetSystemLibrary.PrintString` "RADIAL"))

(fn `CalculateDamage`
  (params (ReceivedDamage :type "Float (double-precision)"))
  (bind _output_get (set `self.DamageAbsorbedByArmor` (/ (`self.Armor`) (- 1.0 (/ (`self.ArmorDamageReduction%`) 100.0)))))
  (bind _returnvalue (- _output_get (`local.ReceivedDamage`)))
  (if (>= _returnvalue 0.0)
    (bind _damage_done_to_armor (`self.DamageArmor` (`local.ReceivedDamage`)))
    (`self.Create Damage Number` _damage_done_to_armor true)
    (elif (< _returnvalue 0.0)
      (if (not (`self.bArmorDestroyed`))
        (`self.DestroyArmor`))
      (bind _damage_done_to_health (`self.DamageHealth` (`local.ReceivedDamage`)))
      (`self.Create Damage Number` _damage_done_to_health)
      (if (<= (`self.Health`) 0.0)
        (`self.EnemyDeath`)))))

(fn `Create Damage Number`
  (params (DamageNumber :type "Float (double-precision)") (IsArmor :type Boolean))
  (bind _returnvalue (`|CreateWidget` "/Game/UI/W_DamageNumber.W_DamageNumber_C" null (`GameplayStatics.ProjectWorldToScreen` (`GameplayStatics.GetPlayerController` 0) (`SceneComponent.K2_GetComponentLocation` (`self.DamageNumberSpawnPoint`))) DamageNumber IsArmor))
  (`UserWidget.AddToViewport` _returnvalue 0))

(fn `DamageArmor`
  (params (`Received Damage` :type "Float (double-precision)"))
  (returns (`Damage Done to Armor` :type "Float (double-precision)"))
  (bind _healthbarref (`self.HealthBarRef`))
  (`KismetSystemLibrary.PrintString` "DamageArmor" true true (struct :`G` 1.0 :`B` 0.065195 :`A` 1.0))
  (bind _output_get (set `self.DamageDoneToArmor` (* (`local.Received Damage`) (- 1.0 (/ (`self.ArmorDamageReduction%`) 100.0)))))
  (bind _output_get_2 (set `self.Armor` (- (`self.Armor`) _output_get)))
  (if (== _output_get_2 0.0)
    (`self.DestroyArmor`))
  (`/Engine/EditorBlueprintResources/StandardMacros.IsValid` _healthbarref
    (:`Is Valid`
      (set `/Game/UI/W_HealthBar.HB_Armor` (`self.Armor`) _healthbarref))
    (:`Is Not Valid`
      _))
  (return _output_get))

(fn `DamageHealth`
  (params (ReceivedDamage :type "Float (double-precision)"))
  (returns (`Damage Done To Health` :type "Float (double-precision)"))
  (bind _healthbarref (`self.HealthBarRef`))
  (bind _output_get (set `self.DamageDoneToHealth` (- (`local.ReceivedDamage`) (`self.DamageAbsorbedByArmor`))))
  (bind _output_get_2 (set `self.Health` (- (`self.Health`) _output_get)))
  (`/Engine/EditorBlueprintResources/StandardMacros.IsValid` _healthbarref
    (:`Is Valid`
      (set `/Game/UI/W_HealthBar.HB_Health` _output_get_2 _healthbarref)
      (return _output_get))))

(fn `DeathDrop`
  (if (> (`KismetMathLibrary.RandomIntegerInRange` 0 100) (- 100 (`self.DropSpawnProbability%`)))
    (for _array_element (`/Game/Core/BP_FirstPersonCharacter.CarriedWeapons` (`/Game/Core/BPFL_MainLibrary.Get Main Character`))
      (`KismetArrayLibrary.Array_Add` (`self.CarriedWeaponClasses`) (`/Game/Gameplay/Weapons/BP_Weapon_Parent.WeaponClass` _array_element)))
    (`|SpawnActorFromClass` "/Game/Gameplay/Weapons/BP_AmmoDrop.BP_AmmoDrop_C" (`self.GetTransform`) "Undefined" "OverrideRootScale" null (`KismetArrayLibrary.Array_Random` (`self.CarriedWeaponClasses`)) null)))

(fn `DestroyArmor`
  (bind _healthbarref (`self.HealthBarRef`))
  (set `self.Armor` 0.0)
  (set `self.bArmorDestroyed` true)
  (`self.Create Damage Number` (`self.DamageAbsorbedByArmor`) true)
  (`/Engine/EditorBlueprintResources/StandardMacros.IsValid` _healthbarref
    (:`Is Valid`
      (set `/Game/UI/W_HealthBar.HB_Armor` 0.0 _healthbarref))))

(fn `EnemyDeath`
  (`/Game/Procedural/BP_SpawnableRoom.Register Enemy Death` (`/Game/Core/BPFL_MainLibrary.GetLastSpawnedRoom`) self)
  (`self.DeathDrop`)
  (`self.K2_DestroyActor`))

(fn `InitiateHealthBar`
  (bind _asw_health_bar (cast `/Game/UI/W_HealthBar` (`WidgetComponent.GetUserWidgetObject` (`self.HealthBar`))))
  (set `self.HealthBarRef` _asw_health_bar)
  (set `/Game/UI/W_HealthBar.HB_MaxHealth` (`self.MaxHealth`) (`self.HealthBarRef`))
  (set `/Game/UI/W_HealthBar.HB_Health` (`self.Health`) (`self.HealthBarRef`))
  (set `/Game/UI/W_HealthBar.HB_MaxArmor` (`self.MaxArmor`) (`self.HealthBarRef`))
  (set `/Game/UI/W_HealthBar.HB_Armor` (`self.Armor`) (`self.HealthBarRef`)))

(fn `InitiateStartValues`
  (set `self.Health` (`self.MaxHealth`))
  (set `self.Armor` (`self.MaxArmor`)))

(fn `RotateHealthBar`
  (bind _healthbar (`self.HealthBar`))
  (bind (_widget _returnvalue) (`/Game/Core/BPFL_MainLibrary.GetWidgetToPlayerRotation` _healthbar))
  (`/Engine/EditorBlueprintResources/StandardMacros.IsValid` _healthbar
    (:`Is Valid`
      (`SceneComponent.K2_SetWorldRotation` _widget _returnvalue false false))))

(fn `UserConstructionScript`)