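; AI Blueprint for a walking enemy that runs the BT_WalkingAI behavior tree from BeginPlay.
; AI Perception updates that involve the first-person player write whether the stimulus was sensed to the CanSeePlayer blackboard key.
; A RotateTowardsPlayer function turns the Cylinder component to face the player pawn, but its call in the event graph is disconnected and never runs.
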(event `self.ReceiveBeginPlay`
  (`AIController.RunBehaviorTree` (`AIBlueprintHelperLibrary.GetAIController` self) "/Game/Gameplay/Enemies/WalkingEnemy/BT_WalkingAI.BT_WalkingAI"))

(event `self.ReceiveTick`
  (params (DeltaSeconds :type "Float (single-precision)")))

(event `self.AIPerception.OnTargetPerceptionUpdated`
  (params (Actor :type "Actor Object Reference") (Stimulus :type "AIStimulus Structure"))
  (cast `/Game/Core/BP_FirstPersonCharacter` Actor)
  (`BlackboardComponent.SetValueAsBool` (`AIBlueprintHelperLibrary.GetBlackboard` null) "CanSeePlayer" (`.bSuccessfullySensed` (break `AIStimulus` Stimulus))))

(fn `RotateTowardsPlayer`
  (bind _cylinder (`self.Cylinder`))
  (`SceneComponent.K2_SetWorldRotation` _cylinder (`KismetMathLibrary.FindLookAtRotation` (`SceneComponent.K2_GetComponentLocation` _cylinder) (`self.K2_GetActorLocation` (`GameplayStatics.GetPlayerPawn` 0))) false false))

(fn `UserConstructionScript`)