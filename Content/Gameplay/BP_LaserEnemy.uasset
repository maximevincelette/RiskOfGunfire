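; BP_LaserEnemy is a laser actor that casts a beam along its forward vector and shows where it hits, with no damage logic.
; Each tick, a debug-drawn Visibility line trace over Distance sets the Niagara beam's end point and a grid-width vector built from beam length and GridSize.
; A second Niagara impact effect moves to the hit location and is visible only while the trace is blocked.
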(event `self.ReceiveBeginPlay`
  (`FXSystemComponent.SetColorParameter` (`self.NiagaraLaser`) "Color" (struct :`R` 0.734375 :`G` 0.18122 :`B` 0.056261 :`A` 1.0))
  (`FXSystemComponent.SetColorParameter` (`self.NiagaraLaserImpact`) "Color" (struct :`R` 1.0 :`G` 0.010197 :`B` 0.030093 :`A` 1.0)))

(event `self.ReceiveTick`
  (params (DeltaSeconds :type "Float (single-precision)"))
  (bind _returnvalue (`self.K2_GetActorLocation`))
  (bind _gridsize (`self.GridSize`))
  (bind _returnvalue_2 (+ _returnvalue (* (`self.GetActorForwardVector`) (`self.Distance`))))
  (set `self.TraceEnd` _returnvalue_2)
  (bind _outhit (`KismetSystemLibrary.LineTraceSingle` :`Start` _returnvalue :`End` _returnvalue_2 :`TraceChannel` "TraceTypeQuery1" :`DrawDebugType` "ForOneFrame"))
  (set `self.bHit` (`GameplayStatics.BreakHitResult` _outhit))
  (set `self.HitLocation` (`.Location` (`GameplayStatics.BreakHitResult` _outhit)))
  (`FXSystemComponent.SetVectorParameter` (`self.NiagaraLaser`) "LaserEnd" (select `bool` (`self.bHit`) :`false` (`self.TraceEnd`) :`true` (`self.HitLocation`)))
  (`FXSystemComponent.SetVectorParameter` (`self.NiagaraLaser`) "LaserEndGridWidth" (select `bool` (`self.bHit`) :`false` (`KismetMathLibrary.MakeVector` (* (`self.Distance`) 0.5) _gridsize _gridsize) :`true` (`KismetMathLibrary.MakeVector` (`KismetMathLibrary.Vector_Distance` (`self.K2_GetActorLocation`) (`self.HitLocation`)) _gridsize _gridsize) :!type "Vector Structure"))
  (`SceneComponent.SetVisibility` (`self.NiagaraLaserImpact`) (`self.bHit`) false)
  (`SceneComponent.K2_SetWorldLocation` (`self.NiagaraLaserImpact`) (`self.HitLocation`) false false))

(fn `UserConstructionScript`)