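; BP_Weapon_Laser is a laser weapon Blueprint that fires a beam for as long as the left mouse button is held.
; Pressing the button prints a debug message, spawns a BP_Laser at SpawnPoint0, stores it and attaches it to that spawn point with relative rules.
; Releasing the button destroys the stored laser instance.
; Input is handled directly through key events, with no active Tick or construction logic.
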(event `Key|LeftMouseButton`
  (params (Key :type "Key Structure"))
  (:`Pressed`
    (`KismetSystemLibrary.PrintString` "Hello")
    (bind _returnvalue (`|SpawnActorFromClass` "/Game/Gameplay/BP_Laser.BP_Laser_C" (`KismetMathLibrary.MakeTransform` (`SceneComponent.K2_GetComponentLocation` (`self.SpawnPoint_0`))) "Undefined" "OverrideRootScale" null null))
    (bind _output_get (set `self.LaserInstance_0` _returnvalue))
    (`self.K2_AttachToComponent` _output_get (`self.SpawnPoint_0`) "None" "KeepRelative" "KeepRelative" "KeepRelative" true))
  (:`Released`
    (`self.K2_DestroyActor` (`self.LaserInstance_0`))))

(fn `UserConstructionScript`
  (`parent.UserConstructionScript`))