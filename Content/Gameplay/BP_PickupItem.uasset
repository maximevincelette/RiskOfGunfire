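; BP_PickupItem is a pickup that shows a stats panel when the player is near and can be taken as the gun.
; A sphere overlap toggles the panel, which Tick turns toward the player while in range and not picked up.
; Interact sets the player's Gun child actor class to its own class, calls the empty TransferStatsToNewChildActor hook, then destroys itself.
; BeginPlay marks child-actor instances as picked up.
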(event `self.ReceiveBeginPlay`
  (set `self.bPickedUp` (`self.IsChildActor`)))

(event `self.ReceiveTick`
  (params (DeltaSeconds :type "Float (single-precision)"))
  (if (`self.IsVisible?`)
    (`/Game/Core/BPFL_MainLibrary.RotateWidgetTowardsPlayer` (`self.ItemStatsPannel`))))

(event `self.Sphere.OnComponentBeginOverlap`
  (params (OverlappedComponent :type "PrimitiveComponent Object Reference") (OtherActor :type "Actor Object Reference") (OtherComp :type "PrimitiveComponent Object Reference") (OtherBodyIndex :type Integer) (bFromSweep :type Boolean) (SweepResult :type "HitResult Structure (by ref)"))
  (cast `/Game/Core/BP_FirstPersonCharacter` OtherActor)
  (bind _output_get (set `self.bInRange` true))
  (`SceneComponent.SetVisibility` (`self.ItemStatsPannel`) _output_get false))

(event `self.Sphere.OnComponentEndOverlap`
  (params (OverlappedComponent :type "PrimitiveComponent Object Reference") (OtherActor :type "Actor Object Reference") (OtherComp :type "PrimitiveComponent Object Reference") (OtherBodyIndex :type Integer))
  (cast `/Game/Core/BP_FirstPersonCharacter` OtherActor)
  (bind _output_get (set `self.bInRange` false))
  (`SceneComponent.SetVisibility` (`self.ItemStatsPannel`) _output_get false))

(event `/Game/FirstPerson/Blueprints/BPI_Interact.Interact`
  (bind _asbp_first_person_character (cast `/Game/Core/BP_FirstPersonCharacter` (`GameplayStatics.GetPlayerCharacter` 0)))
  (`ChildActorComponent.SetChildActorClass` (`/Game/Core/BP_FirstPersonCharacter.Gun` _asbp_first_person_character) (`GameplayStatics.GetObjectClass` self))
  (`self.TransferStatsToNewChildActor`)
  (`self.K2_DestroyActor`))

(fn `IsVisible?`
  (returns (`Visible?` :type Boolean))
  (return (and (not (`self.bPickedUp`)) (`self.bInRange`))))

(fn `TransferStatsToNewChildActor`)

(fn `UserConstructionScript`)