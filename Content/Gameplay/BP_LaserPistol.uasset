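; Laser pistol pickup that attaches to the first-person character's GripPoint socket when the character overlaps its sphere.
; On pickup it subscribes to the character's use-item and stop-using-item dispatchers.
; Firing spawns a Niagara laser system at the spawn point along the camera rotation, with zero particle velocity.
; Both fire and stop check LaserInstance, which stop destroys, but the spawned system is never stored in it.
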(event `self.SphereCollision.OnComponentBeginOverlap`
  (params (OverlappedComponent :type "PrimitiveComponent Object Reference") (OtherActor :type "Actor Object Reference") (OtherComp :type "PrimitiveComponent Object Reference") (OtherBodyIndex :type Integer) (bFromSweep :type Boolean) (SweepResult :type "HitResult Structure (by ref)"))
  (bind _asbp_first_person_character (cast `/Game/FirstPerson/Blueprints/BP_FirstPersonCharacter` OtherActor))
  (bind _output_get (set `self.FirstPersonCharacterRef` _asbp_first_person_character))
  (`self.K2_AttachToComponent` self (`/Game/FirstPerson/Blueprints/BP_FirstPersonCharacter.FirstPersonMesh` _output_get) "GripPoint" "SnapToTarget" "SnapToTarget" "SnapToTarget" true)
  (add `/Game/FirstPerson/Blueprints/BP_FirstPersonCharacter.OnUseItem` (`self.FirstPersonCharacterRef`) (`|CreateDelegate` :!event `OnFireProjectile`))
  (add `/Game/FirstPerson/Blueprints/BP_FirstPersonCharacter.OnStopUsingItem` (`self.FirstPersonCharacterRef`) (`|CreateDelegate` :!event `OnStopFiring`)))

(event `OnFireProjectile`
  ;[1 1 1] Fire projectile
  (if (not (`KismetSystemLibrary.IsValid` (`self.LaserInstance`)))
    (bind _returnvalue (`NiagaraFunctionLibrary.SpawnSystemAtLocation` "/Game/Effects/NE_LaserPistol_System.NE_LaserPistol_System" (`SceneComponent.K2_GetComponentLocation` (`self.SpawnPoint`)) (`PlayerCameraManager.GetCameraRotation` (`GameplayStatics.GetPlayerCameraManager` 0))))
    (`FXSystemComponent.SetVectorParameter` _returnvalue "ParticleVelocity" (0.0 0.0 0.0))))

(event `OnStopFiring`
  (if (`KismetSystemLibrary.IsValid` (`self.LaserInstance`))
    (`self.K2_DestroyActor` (`self.LaserInstance`))))

(fn `UserConstructionScript`)