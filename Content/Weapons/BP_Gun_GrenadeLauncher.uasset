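; BP_Gun_GrenadeLauncher is a grenade launcher weapon that extends a parent gun class and fires one grenade each time shooting starts.
; FireBullet requires a BP_FirstPersonCharacter parent actor and available ammo, then spawns a scaled-down BP_Projectile_Grenade at the barrel and decrements the count.
; An impulse on the grenade's sphere launches it along the camera's aim, or along the barrel's rotation when AlternateFiring is set.
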(event `self.StartShooting`
  (`parent.StartShooting`)
  (`self.FireBullet`))

(event `self.StopShooting`
  (`parent.StopShooting`))

(fn `FireBullet`
  (bind _asbp_first_person_character (cast `/Game/Core/BP_FirstPersonCharacter` (`self.GetParentActor`)))
  (if (> (`self.AmmoCount`) 0)
    (if (`self.bAlternateFiring`)
      (set `self.Direction` (`SceneComponent.K2_GetComponentRotation` (`self.Barrel_RefPoint`)))
      (else
        (set `self.Direction` (`SceneComponent.K2_GetComponentRotation` (`/Game/Core/BP_FirstPersonCharacter.FirstPersonCamera` _asbp_first_person_character)))))
    (bind _returnvalue (`|SpawnActorFromClass` "/Game/Weapons/Projectiles/BP_Projectile_Grenade.BP_Projectile_Grenade_C" (`KismetMathLibrary.MakeTransform` (`SceneComponent.K2_GetComponentLocation` (`self.Barrel_RefPoint`)) (`self.Direction`) (0.1 0.1 0.1)) "Undefined" "OverrideRootScale" null null))
    (`PrimitiveComponent.AddImpulse` (`/Game/Weapons/Projectiles/BP_Projectile_Grenade.Sphere` _returnvalue) (* (`KismetMathLibrary.Normal` (`KismetMathLibrary.GetForwardVector` (`self.Direction`))) (`self.BulletSpeed`)) "None" false)
    (`/Engine/EditorBlueprintResources/StandardMacros.DecrementInt` (`self.AmmoCount`))))

(fn `UserConstructionScript`
  (`parent.UserConstructionScript`))