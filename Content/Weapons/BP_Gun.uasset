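; Gun Blueprint attached under the first-person character that spawns projectiles and tracks magazine and reserve ammo.
; Start/stop events only set Firing and AlternateFiring flags; nothing here calls FireBullet.
; FireBullet spawns a projectile at the barrel, aimed by camera rotation or, in alternate fire, barrel rotation, applies BulletSpeed and decrements ammo.
; ReloadGun refills the magazine from the reserve, handling partial reloads.
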(event `StartShooting`
  (set `self.bFiring` true))

(event `StopShooting`
  (set `self.bFiring` false))

(event `StartAlternateFire`
  (set `self.bAlternateFiring` true))

(event `StopAlternateFire`
  (set `self.bAlternateFiring` false))

(fn `FireBullet`
  (bind _asbp_first_person_character (cast `/Game/Core/BP_FirstPersonCharacter` (`self.GetParentActor`)))
  (if (> (`self.AmmoCount`) 0)
    (if (`self.bAlternateFiring`)
      (set `self.Direction` (`SceneComponent.K2_GetComponentRotation` (`self.Barrel_RefPoint`)))
      (else
        (set `self.Direction` (`SceneComponent.K2_GetComponentRotation` (`/Game/Core/BP_FirstPersonCharacter.FirstPersonCamera` _asbp_first_person_character)))))
    (bind _returnvalue (`|SpawnActorFromClass` "/Game/FirstPerson/Blueprints/BP_FirstPersonProjectile.BP_FirstPersonProjectile_C" (`KismetMathLibrary.MakeTransform` (`SceneComponent.K2_GetComponentLocation` (`self.Barrel_RefPoint`)) (`self.Direction`)) "Undefined" "OverrideRootScale" null null))
    (bind _projectilemovement (`/Game/FirstPerson/Blueprints/BP_FirstPersonProjectile.ProjectileMovement` _returnvalue))
    (set `ProjectileMovementComponent.InitialSpeed` (`self.BulletSpeed`) _projectilemovement)
    (set `ProjectileMovementComponent.MaxSpeed` (`self.BulletSpeed`) _projectilemovement)
    (`/Engine/EditorBlueprintResources/StandardMacros.DecrementInt` (`self.AmmoCount`))))

(fn `ReloadGun`
  (locals (BulletDifference :type Integer))
  (bind _output_get (set `local.BulletDifference` (- (`self.MagSize`) (`self.AmmoCount`))))
  (if (>= (`self.AmmoMax`) _output_get)
    (set `self.AmmoCount` (`self.MagSize`))
    (set `self.AmmoMax` (- (`self.AmmoMax`) (`local.BulletDifference`)))
    (else
      (set `self.AmmoCount` (+ (`self.AmmoCount`) (`self.AmmoMax`)))
      (set `self.AmmoMax` 0))))

(fn `UserConstructionScript`
  (`parent.UserConstructionScript`))