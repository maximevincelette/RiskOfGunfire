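; Charged gun Blueprint, a child weapon that builds charge while shooting is held and fires on release.
; A timeline paced by ChargeTime drives CurrentCharge and auto-releases at full charge; stopping fires if the charge meets a minimum threshold.
; The timeline then reverses at normal rate, and a new charge requires a low CurrentCharge.
; FireBullet scales BulletSpeed by charge around the parent call, then resets it to a hardcoded value.
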(event `self.StartShooting`
  (`parent.StartShooting`)
  (if (and (not (`self.bCharging`)) (<= (`self.CurrentCharge`) 0.2))
    (set `self.bCharging` true)
    (`TimelineComponent.SetPlayRate` (`self.ChargeWeaponTL`) (/ 1.0 (`self.ChargeTime`)))
    (bind (_direction _weaponcharge) (`Timeline|ChargeWeaponTL` :!label _label)
      (:`Update`
        (bind _output_get (set `self.CurrentCharge` (`KismetMathLibrary.FClamp` _weaponcharge)))
        (`KismetSystemLibrary.PrintString` (`KismetStringLibrary.Conv_DoubleToString` _output_get) true true (struct :`G` 0.66 :`B` 1.0 :`A` 1.0) 0.0)
        (if (>= _output_get 1.0)
          (`self.StopShooting`))))))

(event `self.StopShooting`
  (`parent.StopShooting`)
  (if (and (`self.bCharging`) (>= (`self.CurrentCharge`) 0.2))
    (`self.FireBullet`))
  (set `self.bCharging` false)
  (`TimelineComponent.SetPlayRate` (`self.ChargeWeaponTL`) 1.0)
  (goto _label :!via `Reverse`))

(fn `FireBullet`
  (set `self.BulletSpeed` (* (`self.BulletSpeed`) (`self.CurrentCharge`)))
  (`parent.FireBullet`)
  (set `self.BulletSpeed` 3000.0))

(fn `UserConstructionScript`
  (`parent.UserConstructionScript`))