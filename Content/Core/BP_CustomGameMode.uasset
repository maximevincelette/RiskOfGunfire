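; BP_CustomGameMode is a game mode that limits how many spawned rooms stay in the level at once.
; AddSpawnedRoomToArray appends each room to SpawnedRooms and, once the count exceeds OldRoomsToKeepSpawned plus one, trims the oldest.
; Trimming removes and destroys that room with its ActorsToDestroy, then closes the AssociatedDoor of the new oldest room.
; BeginPlay, Tick and the construction script are empty.
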(fn `AddSpawnedRoomToArray`
  (params (RoomToAddToArray :type "/Game/Procedural/BP_SpawnableRoom Object Reference"))
  (bind _spawnedrooms (`self.SpawnedRooms`))
  (`KismetArrayLibrary.Array_Add` _spawnedrooms RoomToAddToArray)
  (if (> (`KismetArrayLibrary.Array_Length` _spawnedrooms) (+ (`self.OldRoomsToKeepSpawned`) 1))
    (`self.DestroyOldestRoomAndDoor`)
    (`self.CloseOldestRemainingDoor`)))

(fn `CloseOldestRemainingDoor`
  (bind _output_get (set `self.DoorToClose` (`/Game/Procedural/BP_SpawnableRoom.AssociatedDoor` (`|GetArrayItem` (`self.SpawnedRooms`)))))
  (`/Game/Procedural/BP_Door.CloseDoor` _output_get))

(fn `DestroyOldestRoomAndDoor`
  (bind _spawnedrooms (`self.SpawnedRooms`))
  (set `self.RoomToDestroy` (`|GetArrayItem` _spawnedrooms))
  (`KismetArrayLibrary.Array_Remove` _spawnedrooms)
  (for _array_element (`/Game/Procedural/BP_SpawnableRoom.ActorsToDestroy` (`self.RoomToDestroy`))
    (`self.K2_DestroyActor` _array_element))
  (`self.K2_DestroyActor` (`self.RoomToDestroy`)))

(fn `UserConstructionScript`)