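; Skill tree component that holds skill points and a map of category names to ordered skill arrays.
; AddSkillArray registers a category, sets its first skill's status to what appears to be unlockable, and binds to each skill's acquire request.
; OnSkillAcquired deducts the cost if points suffice, updates that skill's status, advances the next one in line and applies the skill to the owner.
; Each category thus unlocks linearly.
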(fn `AddPoints`
  (params (PointsToAdd :type Integer))
  (set `self.Points` (+ PointsToAdd (`self.Points`))))

(fn `AddSkillArray`
  (params (Category :type String) (Skills :type "Array of /Game/Core/BP_Skill Object Reference"))
  (if (> (`KismetArrayLibrary.Array_Length` Skills) 0)
    (`|ExecutionSequence`
      (:`then_0`
        (`/Game/Core/BP_Skill.SetStatus` (`|GetArrayItem` (`local.Skills`)) "NewEnumerator2")
        (`BlueprintMapLibrary.Map_Add` (`self.Root`) (`local.Category`) (make `/Game/Core/S_SkillAray` (`local.Skills`))))
      (:`then_1`
        (for _array_element (`local.Skills`)
          (add `/Game/Core/BP_Skill.OnAcquireRequest` _array_element (`|CreateDelegate` :!event `OnSkillAcquired`)))))))

(fn `GetCategories`
  (returns (Keys :type "Array of String"))
  (bind _keys (`BlueprintMapLibrary.Map_Keys` (`self.Root`)))
  (return _keys))

(fn `GetSkillArray`
  (params (CategoryName :type String))
  (returns (Value :type "/Game/Core/S_SkillAray Structure") (`Found?` :type Boolean))
  (if (`BlueprintMapLibrary.Map_Contains` (`self.Root`) CategoryName)
    (return (`BlueprintMapLibrary.Map_Find` (`self.Root`) (`local.CategoryName`)) true)
    (else
      (return (struct) false))))

(fn `OnSkillAcquired`
  (params (Category :type String) (SkillAcquired :type "/Game/Core/BP_Skill Object Reference"))
  (locals (`Index (local)` :type Integer :default 0))
  (bind _skills (break `/Game/Core/S_SkillAray` (`BlueprintMapLibrary.Map_Find` (`self.Root`) (`local.Category`))))
  (if (>= (`self.Points`) (`/Game/Core/BP_Skill.Cost` SkillAcquired))
    (set `self.Points` (- (`self.Points`) (`/Game/Core/BP_Skill.Cost` (`local.SkillAcquired`))))
    (`|ExecutionSequence`
      (:`then_0`
        (set `local.Index (local)` (`KismetArrayLibrary.Array_Find` _skills (`local.SkillAcquired`)))
        (if (`KismetArrayLibrary.Array_IsValidIndex` _skills (`local.Index (local)`))
          (`/Game/Core/BP_Skill.SetStatus` (`|GetArrayItem` _skills (`local.Index (local)`)) "NewEnumerator1")
          (`/Engine/EditorBlueprintResources/StandardMacros.IncrementInt` (`local.Index (local)`)
            (:`  `
              (if (`KismetArrayLibrary.Array_IsValidIndex` _skills (`local.Index (local)`))
                (`/Game/Core/BP_Skill.SetStatus` (`|GetArrayItem` _skills (`local.Index (local)`)) "NewEnumerator2"))))))
      (:`then_1`
        (`/Game/Core/BP_Skill.ApplySkill` (`local.SkillAcquired`) (`self.GetOwner`))))))